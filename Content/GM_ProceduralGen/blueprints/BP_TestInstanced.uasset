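; BP_TestInstanced is a test actor that scatters thousands of copies of a randomly chosen mesh around its origin.
; Its construction script picks one mesh from PossibleMeshes for the InstancedStaticMesh component, then loops to add instances at random directions and distances within a small radius.
; Each iteration also prints a freshly drawn random PossibleMeshes index, unrelated to the mesh in use.
; The event graph holds only disabled placeholder events.
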(event EventBeginPlay)

(event Collision|EventActorBeginOverlap
  (params (OtherActor :type Actor%20Object%20Reference)))

(event EventTick
  (params (DeltaSeconds :type Float%20%28single-precision%29)))

(fn ConstructionScript
  (bind _possiblemeshes (Variables|Default|GetPossibleMeshes))
  (bind (_outitem _outindex) (Utilities|Array|Random _possiblemeshes))
  (Components|StaticMesh|SetStaticMesh (Variables|Default|GetInstancedStaticMesh) (.mesh (Utilities|Struct|BreakSObjectInfo _outitem)))
  (for _index (range 0 10000)
    (bind _returnvalue (Components|InstancedStaticMesh|AddInstance (Variables|Default|GetInstancedStaticMesh) (Math|Conversions|ToTransform(Vector) (* (Math|Random|RandomUnitVector) (* (Math|Random|RandomFloat) 1e+02)))))
    (Development|PrintString (Utilities|String|ToString(Integer) _outindex))))