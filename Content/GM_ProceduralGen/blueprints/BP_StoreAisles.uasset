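; Procedural store aisle generator that spawns rows of BP_Shelf actors, sized from grid dimensions and spaced by aisle width, with alternating shelves flipped.
; The construction script clears and spawns all rows at once, while RegenerateAtSize rebuilds at new dimensions one shelf per Tick.
; Each spawned shelf starts its own gradual generation, and the generator signals every step and completion.
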(event EventBeginPlay
  (Generate|CalculateGenerateCounts))

(event Collision|EventActorBeginOverlap
  (params (OtherActor :type Actor%20Object%20Reference)))

(event EventTick
  (params (DeltaSeconds :type Float%20%28single-precision%29))
  (if (Variables|Generate|GetIsGraduallyGenerating)
    (Generate|GradualGenerateStep)
    (Generate|CheckGradualGenerateComplete)))

(fn ConstructionScript
  (Generate|ClearAllGenerated)
  (Generate|CalculateGenerateCounts)
  (Generate|GenerateImmediately))

(fn CalculateGenerateCounts
  (Variables|Generate|SetShelfCount (- (* (Variables|Config|GetYSize) 2) 1))
  (Variables|Generate|SetShelfLength (- (* (Variables|Config|GetXSize) 2) 1)))

(fn GenerateImmediately
  (bind _shelfcount (Variables|Generate|GetShelfCount))
  (bind _returnvalue (- _shelfcount 1))
  (for _index (range 0 _returnvalue)
    (Generate|GenerateShelf _index)
    (Default|CallGenerationStep _index _returnvalue))
  (Default|CallGenerationComplete))

(fn ClearAllGenerated
  (bind _spawnedshelflist (Variables|Default|GetSpawnedShelfList))
  (Development|PrintString (Utilities|String|ToString(Integer) (Utilities|Array|Length _spawnedshelflist)))
  (for _array_element _spawnedshelflist
    (Development|PrintString (Utilities|GetObjectName _array_element))
    (Actor|DestroyActor _array_element))
  (Utilities|Array|Clear _spawnedshelflist))

(fn GenerateShelf
  (params (Index :type Integer))
  (bind _defaultsceneroot (Variables|Default|GetDefaultSceneRoot))
  (bind _returnvalue (Transformation|GetRelativeTransform _defaultsceneroot))
  (bind _returnvalue_2 (Game|SpawnActorfromClass "/Game/GM_ProceduralGen/blueprints/BP_Shelf.BP_Shelf_C" (Math|Transform|MakeTransform (Math|Vector|MakeVector (+ (.x (.location _returnvalue)) 2e+02) (+ (Math|Conversions|ToFloat(Integer) (* (/ (+ Index 1) 2) (Variables|Config|GetAisleWidth))) (.y (.location _returnvalue))) (.z (.location _returnvalue))) (.rotation _returnvalue) "1,1,1") "Undefined" 0 (Variables|Generate|GetShelfLength) (!= (Math|Integer|%(Integer) Index 2) 0) false 0))
  (Utilities|Array|Add (Variables|Default|GetSpawnedShelfList) _returnvalue_2)
  (Default|StartGradualGenerate _returnvalue_2))

(fn GradualGenerateStep
  (Generate|GenerateShelf (Variables|Generate|GetCurrentGradualGenerateIndex))
  (Default|CallGenerationStep (Variables|Generate|GetCurrentGradualGenerateIndex) (- (Variables|Generate|GetShelfCount) 1))
  (Variables|Generate|SetCurrentGradualGenerateIndex (+ (Variables|Generate|GetCurrentGradualGenerateIndex) 1)))

(fn StartGradualGenerate
  (if (not (Variables|Generate|GetIsGraduallyGenerating))
    (Generate|ClearAllGenerated)
    (Variables|Generate|SetCurrentGradualGenerateIndex 0)
    (Variables|Generate|SetIsGraduallyGenerating true)))

(fn CheckGradualGenerateComplete
  (if (Variables|Generate|GetIsGraduallyGenerating)
    (bind _output_get (Variables|Generate|SetIsGraduallyGenerating (<= (Variables|Generate|GetCurrentGradualGenerateIndex) (Variables|Generate|GetShelfCount))))
    (if (not _output_get)
      (Default|CallGenerationComplete))))

(fn RegenerateatSize
  (params (XSize :type Integer) (YSize :type Integer) (AisleWidth :type Integer))
  (if (not (Variables|Generate|GetIsGraduallyGenerating))
    (Variables|Config|SetXSize XSize)
    (Variables|Config|SetYSize YSize)
    (Variables|Config|SetAisleWidth AisleWidth)
    (Generate|CalculateGenerateCounts)
    (Generate|StartGradualGenerate)))