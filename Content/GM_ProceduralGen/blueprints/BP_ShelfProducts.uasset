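; Procedural shelf filler that packs a box volume with rows and stacks of product meshes, one section per mesh type.
; Construction creates an instanced static mesh component per product and measures its bounds.
; CalculateLayout derives per-section width, depth and height counts from those sizes and the gap.
; GenerateSection spawns BP_ShelfProductsSection actors to place instances, either all at once or one per tick with step and completion events.
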(event EventBeginPlay
  (if (Variables|Generate|GetShouldGenerateImmediately)
    (Generate|GenerateImmediately)))

(event Collision|EventActorBeginOverlap
  (params (OtherActor :type Actor%20Object%20Reference)))

(event EventTick
  (params (DeltaSeconds :type Float%20%28single-precision%29))
  (if (Variables|Generate|GetIsGraduallyGenerating)
    (Generate|GradualGenerateStep)
    (Generate|CheckGradualGenerateComplete)))

(fn ConstructionScript
  (bind _productmeshes (Variables|Meshes|GetProductMeshes))
  (Utilities|FlowControl|Sequence
    (:then_0
      (for _array_element _productmeshes
        (bind (_instance _size) (Config|InitMesh _array_element))
        (Utilities|Array|Add (Variables|MeshInstance|GetMeshes) _instance)
        (Utilities|Array|Add (Variables|Measurements|GetProductSizes) _size))
      (Variables|Config|SetSectionCount (- (Utilities|Array|Length _productmeshes) 1)))
    (:then_1
      (Generate|ClearAllPlacedInstances)
      (if (Variables|Generate|GetShouldGenerateImmediately)
        (Generate|GenerateImmediately)))))

(fn InitMesh
  (params (Mesh :type Static%20Mesh%20Object%20Reference))
  (bind _returnvalue (AddComponent|AddInstancedStaticMeshComponent false))
  (Components|StaticMesh|SetStaticMesh _returnvalue Mesh)
  (bind _size (Utility|MeasureMesh Mesh))
  (return _returnvalue _size))

(fn MeasureMesh
  (params (mesh :type Static%20Mesh%20Object%20Reference))
  (bind _returnvalue (StaticMesh|GetBoundingBox mesh))
  (bind (_min _max) (Utilities|Struct|BreakBox _returnvalue))
  (bind _returnvalue_2 (AddComponent|AddStaticMeshComponent false))
  (Components|StaticMesh|SetStaticMesh _returnvalue_2 mesh)
  (bind _output_get (LocalVariables|SetMeshSize (- _max _min)))
  (Components|DestroyComponent _returnvalue_2)
  (return _output_get))

(fn ClearAllPlacedInstances
  (for _array_element (Variables|MeshInstance|GetMeshes)
    (Components|InstancedStaticMesh|ClearInstances _array_element)))

(fn GenerateImmediately
  (Generate|ClearAllPlacedInstances)
  (Generate|CalculateLayout)
  (for (_ _array_index) (Variables|MeshInstance|GetMeshes)
    (Generate|GenerateSection _array_index)))

(fn CalculateLayout
  (bind _size (Variables|Config|GetSize))
  (Utilities|Array|Clear (Variables|Config|GetSectionWidthCounts))
  (Utilities|Array|Clear (Variables|Config|GetSectionDepthCounts))
  (Utilities|Array|Clear (Variables|Config|GetSectionHeightCounts))
  (LocalVariables|SetFilledSpace 0.0)
  (LocalVariables|SetSectionWidthStandard (/ (.x (Variables|Config|GetSize)) (Utilities|Array|Length (Variables|MeshInstance|GetMeshes))))
  (for (_array_element _array_index) (Variables|Measurements|GetProductSizes)
    (Utilities|FlowControl|Sequence
      (:then_0
        (bind _output_get (LocalVariables|SetFilledSpace (+ (LocalVariables|GetFilledSpace) (* (Math|Conversions|ToFloat(Integer) (Math|Float|Floor (/ (LocalVariables|GetSectionWidthStandard) (+ (.x _array_element) (Variables|Config|GetObjectGap))))) (+ (.x _array_element) (Variables|Config|GetObjectGap))))))
        (Utilities|Array|Add (Variables|Config|GetSectionWidthCounts) (Math|Integer|SelectInt (Math|Float|Floor (/ (LocalVariables|GetSectionWidthStandard) (+ (.x _array_element) (Variables|Config|GetObjectGap)))) (Math|Float|Truncate (/ (Math|Float|SelectFloat _output_get (* (Math|Conversions|ToFloat(Integer) (Math|Float|Floor (/ (LocalVariables|GetSectionWidthStandard) (+ (.x _array_element) (Variables|Config|GetObjectGap))))) (+ (.x _array_element) (Variables|Config|GetObjectGap))) (< (* (Math|Conversions|ToFloat(Integer) (Math|Float|Floor (/ (LocalVariables|GetSectionWidthStandard) (+ (.x _array_element) (Variables|Config|GetObjectGap))))) (+ (.x _array_element) (Variables|Config|GetObjectGap))) _output_get)) (+ (.x _array_element) (Variables|Config|GetObjectGap)))) (!= _array_index (Variables|Config|GetSectionCount)))))
      (:then_1
        (Utilities|Array|Add (Variables|Config|GetSectionDepthCounts) (Math|Float|Truncate (/ (.y _size) (+ (.y _array_element) (Variables|Config|GetObjectGap))))))
      (:then_2
        (Utilities|Array|Add (Variables|Config|GetSectionHeightCounts) (Math|Integer|Max(Integer) (Math|Float|Truncate (/ (.z _size) (.z _array_element))) 1))))))

(fn GenerateSection
  (params (Index :type Integer))
  (LocalVariables|SetCurrentSectionStartX 0.0)
  (bind (_array_element _array_index) (Utilities|Array|ForEachLoopwithBreak (Variables|Config|GetSectionWidthCounts) :!label _label)
    (:LoopBody
      (if (< _array_index Index)
        (LocalVariables|SetCurrentSectionStartX (+ (LocalVariables|GetCurrentSectionStartX) (* (+ (Variables|Config|GetObjectGap) (.x (Utilities|Array|Get(acopy) (Variables|Measurements|GetProductSizes) _array_index))) _array_element)))
        (else
          (goto _label Break))))
    (:Completed
      (bind _returnvalue (Game|SpawnActorfromClass "/Game/GM_ProceduralGen/blueprints/BP_ShelfProductsSection.BP_ShelfProductsSection_C" (Transformation|GetRelativeTransform (Variables|Default|GetDefaultSceneRoot)) "AlwaysSpawn" 0 (Variables|Config|GetObjectGap) (Variables|Config|GetVariance) (- (Utilities|Array|Get(acopy) (Variables|Config|GetSectionWidthCounts) Index) 1) (- (Utilities|Array|Get(acopy) (Variables|Config|GetSectionDepthCounts) Index) 1) (- (Utilities|Array|Get(acopy) (Variables|Config|GetSectionHeightCounts) Index) 1) (Utilities|Array|Get(acopy) (Variables|MeshInstance|GetMeshes) Index) (Utilities|Array|Get(acopy) (Variables|Measurements|GetProductSizes) Index) (Variables|Generate|GetShouldGenerateImmediately) (Math|Vector|MakeVector (LocalVariables|GetCurrentSectionStartX) 0.0 0.0) 0))
      (Default|StartGradualGenerate _returnvalue))))

(fn StartGradualGenerate
  (if (not (Variables|Generate|GetIsGraduallyGenerating))
    (Generate|ClearAllPlacedInstances)
    (Generate|CalculateLayout)
    (Variables|Generate|SetCurrentGradualGenerateIndex 0)
    (Variables|Generate|SetIsGraduallyGenerating true)))

(fn GradualGenerateStep
  (Generate|GenerateSection (Variables|Generate|GetCurrentGradualGenerateIndex))
  (Default|CallGenerationStep (Variables|Generate|GetCurrentGradualGenerateIndex) (Variables|Config|GetSectionCount))
  (Variables|Generate|SetCurrentGradualGenerateIndex (+ (Variables|Generate|GetCurrentGradualGenerateIndex) 1)))

(fn CheckGradualGenerateComplete
  (if (Variables|Generate|GetIsGraduallyGenerating)
    (bind _output_get (Variables|Generate|SetIsGraduallyGenerating (< (Variables|Generate|GetCurrentGradualGenerateIndex) (Variables|Config|GetSectionCount))))
    (if (not _output_get)
      (Default|CallGenerationComplete))))