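; BP_StoreShell procedurally builds a rectangular store shell of corners, walls, floor, ceiling and ceiling lights on an XSize by YSize grid.
; Construction measures each mesh's bounds and places pieces immediately as instanced meshes, except lights, which become individual tracked components.
; Regenerating at a given or random size clears the shell and rebuilds it one index per Tick through the same placement functions, then signals completion.
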(event EventBeginPlay
  (Input|EnableInput (Class|GameplayStatics|GetPlayerControllerfromID)))

(event EventTick
  (params (DeltaSeconds :type Float%20%28single-precision%29))
  (if (Variables|Generate|GetIsGraduallyGenerating)
    (Generate|GradualGenerateStep)
    (Generate|CheckGradualGenerateComplete)))

(fn ConstructionScript
  (Utilities|FlowControl|Sequence
    (:then_0
      (bind (_instance _size) (Setup|InitMesh (Variables|Meshes|GetCornerMesh)))
      (Variables|MeshInstance|SetCorner _instance)
      (Variables|Measurements|SetCornerSize _size)
      (bind (_instance_2 _size_2) (Setup|InitMesh (Variables|Meshes|GetWallMesh)))
      (Variables|MeshInstance|SetWall _instance_2)
      (Variables|Measurements|SetWallSize _size_2)
      (bind (_instance_3 _size_3) (Setup|InitMesh (Variables|Meshes|GetFloorMesh)))
      (Variables|MeshInstance|SetFloor _instance_3)
      (Variables|Measurements|SetFloorSize _size_3)
      (bind (_instance_4 _size_4) (Setup|InitMesh (Variables|Meshes|GetCeilingMesh)))
      (Variables|MeshInstance|SetCeiling _instance_4)
      (Variables|Measurements|SetCeilingSize _size_4)
      (bind (_instance_5 _size_5) (Setup|InitMesh (Variables|Meshes|GetCeilingLightMesh)))
      (Variables|MeshInstance|SetCeilingLight _instance_5)
      (Variables|Measurements|SetCeilingLightSize _size_5))
    (:then_1
      (Generate|ClearAllPlacedInstancesandMeshes)
      (Generate|GenerateImmediately))))

(fn MeasureMesh
  (params (Mesh :type Static%20Mesh%20Object%20Reference))
  (bind _returnvalue (StaticMesh|GetBoundingBox Mesh))
  (bind (_min _max) (Utilities|Struct|BreakBox _returnvalue))
  (bind _returnvalue_2 (AddComponent|AddStaticMeshComponent false))
  (Components|StaticMesh|SetStaticMesh _returnvalue_2 Mesh)
  (bind _output_get (LocalVariables|SetMeshSize (- _max _min)))
  (Components|DestroyComponent _returnvalue_2)
  (return _output_get))

(fn InitMesh
  (params (mesh :type Static%20Mesh%20Object%20Reference))
  (bind _returnvalue (AddComponent|AddInstancedStaticMeshComponent false))
  (Components|StaticMesh|SetStaticMesh _returnvalue mesh)
  (bind _size (Utility|MeasureMesh mesh))
  (return _returnvalue _size))

(fn ClearAllPlacedInstancesandMeshes
  (bind _addedstaticmeshes (Variables|Meshes|GetAddedStaticMeshes))
  (Components|InstancedStaticMesh|ClearInstances (Variables|MeshInstance|GetCorner))
  (Components|InstancedStaticMesh|ClearInstances (Variables|MeshInstance|GetWall))
  (Components|InstancedStaticMesh|ClearInstances (Variables|MeshInstance|GetFloor))
  (Components|InstancedStaticMesh|ClearInstances (Variables|MeshInstance|GetCeiling))
  (for _array_element _addedstaticmeshes
    (Components|DestroyComponent _array_element))
  (Utilities|Array|Clear _addedstaticmeshes))

(fn GenerateImmediately
  (Utilities|FlowControl|Sequence
    (:then_0
      (Generate|CalculateGenerateCounts))
    (:then_1
      (for _index (range (Variables|Generate|GetGenerateWallYMin) (Variables|Generate|GetGenerateWallYMax))
        (Generate|GenerateWallYAxis _index)))
    (:then_2
      (for _index_2 (range (Variables|Generate|GetGenerateWallXMin) (Variables|Generate|GetGenerateWallXMax))
        (Generate|GenerateWallXAxis _index_2)))
    (:then_3
      (for _index_3 (range 0 (Variables|Generate|GetGenerateCeilingMax))
        (Generate|GenerateFloorCeiling _index_3)))))

(fn GenerateWallYAxis
  (params (Index :type Integer))
  (bind _returnvalue (== Index 1))
  (bind _xsize (Variables|Config|GetXSize))
  (bind _ysize (Variables|Config|GetYSize))
  (bind _corner (Variables|MeshInstance|GetCorner))
  (bind _wall (Variables|MeshInstance|GetWall))
  (bind _wallsize (Variables|Measurements|GetWallSize))
  (bind _returnvalue_2 (== Index _ysize))
  (bind _returnvalue_3 (- _xsize 1))
  (bind _returnvalue_4 (* (.y _wallsize) Index))
  (bind _returnvalue_5 (== Index _ysize))
  (bind _returnvalue_6 (* (.y _wallsize) -1.0))
  (bind _returnvalue_7 (Math|Vector|MakeVector 0.0 _returnvalue_4 0.0))
  (bind _returnvalue_8 (or _returnvalue _returnvalue_2))
  (bind _returnvalue_9 (* _returnvalue_3 (.y _wallsize)))
  (bind _returnvalue_10 (Math|Vector|MakeVector _returnvalue_9 _returnvalue_6 0.0))
  (bind _returnvalue_11 (select _returnvalue_8 _corner _wall))
  (bind _returnvalue_12 (+ _returnvalue_7 _returnvalue_10))
  (Components|InstancedStaticMesh|AddInstance _returnvalue_11 (Math|Transform|MakeTransform (select _returnvalue_5 (+ _returnvalue_7 (Math|Vector|MakeVector (.y _wallsize) 0.0 0.0)) _returnvalue_7) (select _returnvalue_5 "0,270.000000, 0" "0, 0, 0")))
  (Components|InstancedStaticMesh|AddInstance _returnvalue_11 (Math|Transform|MakeTransform (Math|Vector|SelectVector _returnvalue_12 (+ _returnvalue_12 (Math|Vector|MakeVector (.y _wallsize) 0.0 0.0)) _returnvalue) (Math|Rotator|CombineRotators (Math|Rotator|MakeRotator 0.0 0.0 1.8e+02) (Math|Rotator|SelectRotator "0,270.000000, 0" "0, 0, 0" _returnvalue)))))

(fn GenerateWallXAxis
  (params (Index :type Integer))
  (bind _returnvalue (Math|Rotator|MakeRotator 0.0 0.0 9e+01))
  (bind _returnvalue_2 (- Index 1))
  (bind _wallsize (Variables|Measurements|GetWallSize))
  (bind _wall (Variables|MeshInstance|GetWall))
  (bind _returnvalue_3 (* _returnvalue_2 (.y _wallsize)))
  (bind _returnvalue_4 (Math|Vector|MakeVector _returnvalue_3 0.0 0.0))
  (Components|InstancedStaticMesh|AddInstance _wall (Math|Transform|MakeTransform _returnvalue_4 _returnvalue))
  (Components|InstancedStaticMesh|AddInstance _wall (Math|Transform|MakeTransform (+ _returnvalue_4 (Math|Vector|MakeVector (* (.y _wallsize) 1.0) (* (.y _wallsize) (Variables|Config|GetYSize)) 0.0)) (Math|Rotator|CombineRotators _returnvalue "0,180.000000, 0"))))

(fn GenerateFloorCeiling
  (params (Index :type Integer))
  (bind _floorsize (Variables|Measurements|GetFloorSize))
  (bind _ysize (Variables|Config|GetYSize))
  (bind _floorsize_2 (Variables|Measurements|GetFloorSize))
  (bind _returnvalue (Math|Integer|%(Integer) Index _ysize))
  (bind _returnvalue_2 (/ Index _ysize))
  (bind _returnvalue_3 (* _returnvalue_2 (.x _floorsize)))
  (bind _returnvalue_4 (* _returnvalue (.y _floorsize)))
  (bind _returnvalue_5 (+ _returnvalue_4 (.y _floorsize)))
  (bind _returnvalue_6 (Math|Vector|MakeVector _returnvalue_3 _returnvalue_5 0.0))
  (bind _returnvalue_7 (Math|Transform|MakeTransform _returnvalue_6))
  (Components|InstancedStaticMesh|AddInstance (Variables|MeshInstance|GetFloor) _returnvalue_7)
  (Components|InstancedStaticMesh|AddInstance (Variables|MeshInstance|GetCeiling) _returnvalue_7)
  (bind _returnvalue_8 (AddComponent|AddStaticMeshComponent false (Math|Transform|MakeTransform (+ (+ _returnvalue_6 (Math|Vector|MakeVector (/ (.x _floorsize_2) 2.0) (* (/ (.y _floorsize_2) 2.0) -1.0) (- (.z (Variables|Measurements|GetWallSize)) 5.0))) (* (Variables|Measurements|GetCeilingLightSize) "0.500000,0.500000,0")))))
  (Utilities|Array|Add (Variables|Meshes|GetAddedStaticMeshes) _returnvalue_8)
  (Components|StaticMesh|SetStaticMesh _returnvalue_8 (Variables|Meshes|GetCeilingLightMesh)))

(fn CalculateGenerateCounts
  (Variables|Generate|SetGenerateWallYMin 1)
  (bind _output_get (Variables|Generate|SetGenerateWallYMax (Variables|Config|GetYSize)))
  (Variables|Generate|SetGenerateWallXMin 2)
  (bind _output_get_2 (Variables|Generate|SetGenerateWallXMax (- (Variables|Config|GetXSize) 1)))
  (bind _output_get_3 (Variables|Generate|SetGenerateCeilingMax (- (* (Variables|Config|GetXSize) (Variables|Config|GetYSize)) 1)))
  (Variables|Generate|SetLargestGenerateIndex (Math|Integer|Max(Integer) _output_get _output_get_2 _output_get_3)))

(fn StartGradualGenerate
  (if (not (Variables|Generate|GetIsGraduallyGenerating))
    (Generate|ClearAllPlacedInstancesandMeshes)
    (Generate|CalculateGenerateCounts)
    (Variables|Generate|SetCurrentGradualGenerateIndex 0)
    (Variables|Generate|SetIsGraduallyGenerating true)))

(fn GradualGenerateStep
  (Utilities|FlowControl|Sequence
    (:then_0
      (if (and (>= (Variables|Generate|GetCurrentGradualGenerateIndex) (Variables|Generate|GetGenerateWallYMin)) (<= (Variables|Generate|GetCurrentGradualGenerateIndex) (Variables|Generate|GetGenerateWallYMax)))
        (Generate|GenerateWallYAxis (Variables|Generate|GetCurrentGradualGenerateIndex))))
    (:then_1
      (if (and (>= (Variables|Generate|GetCurrentGradualGenerateIndex) (Variables|Generate|GetGenerateWallXMin)) (<= (Variables|Generate|GetCurrentGradualGenerateIndex) (Variables|Generate|GetGenerateWallXMax)))
        (Generate|GenerateWallXAxis (Variables|Generate|GetCurrentGradualGenerateIndex))))
    (:then_2
      (if (<= (Variables|Generate|GetCurrentGradualGenerateIndex) (Variables|Generate|GetGenerateCeilingMax))
        (Generate|GenerateFloorCeiling (Variables|Generate|GetCurrentGradualGenerateIndex))))
    (:then_3
      (Variables|Generate|SetCurrentGradualGenerateIndex (+ (Variables|Generate|GetCurrentGradualGenerateIndex) 1)))))

(fn CheckGradualGenerateComplete
  (if (Variables|Generate|GetIsGraduallyGenerating)
    (bind _output_get (Variables|Generate|SetIsGraduallyGenerating (<= (Variables|Generate|GetCurrentGradualGenerateIndex) (Variables|Generate|GetLargestGenerateIndex))))
    (if (not _output_get)
      (Default|CallGenerationComplete))))

(fn GetSize
  (bind _wallsize (Variables|Measurements|GetWallSize))
  (return (Math|Vector|MakeVector (* (.y _wallsize) (Variables|Config|GetXSize)) (* (.y _wallsize) (Variables|Config|GetYSize)) (.z _wallsize))))

(fn RegenerateatSize
  (params (XSize :type Integer) (YSize :type Integer))
  (if (not (Variables|Generate|GetIsGraduallyGenerating))
    (Variables|Config|SetXSize XSize)
    (Variables|Config|SetYSize YSize)
    (Generate|StartGradualGenerate)))

(fn RegenerateRandom
  (Generate|RegenerateatSize (Math|Random|RandomIntegerinRange 2 8) (Math|Random|RandomIntegerinRange 2 8)))