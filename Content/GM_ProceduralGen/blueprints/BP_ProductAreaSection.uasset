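; BP_ProductAreaSection procedurally fills a product area with stacked rows of one mesh, using an instanced static mesh component.
; Instances form a width, depth and height grid spaced by size and gap, with random offset and yaw variation and optional Y flipping.
; It generates all at once in construction and BeginPlay, or clears and rebuilds one width step per Tick, firing step and completion calls.
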(event EventBeginPlay
  (if (Variables|Generate|GetShouldGenerateImmediately)
    (Generate|GenerateImmediately)))

(event Collision|EventActorBeginOverlap
  (params (OtherActor :type Actor%20Object%20Reference)))

(event EventTick
  (params (DeltaSeconds :type Float%20%28single-precision%29))
  (if (Variables|Generate|GetIsGraduallyGenerating)
    (Generate|GradualGenerateStep)
    (Generate|CheckGradualGenerateComplete)))

(fn ConstructionScript
  (bind _instancesize (Variables|Measurements|GetInstanceSize))
  (bind _objectgap (Variables|Config|GetObjectGap))
  (Variables|Measurements|SetInstanceArea (Math|Vector|MakeVector (+ (.x _instancesize) _objectgap) (+ (.y _instancesize) _objectgap) (.z _instancesize)))
  (bind _returnvalue (AddComponent|AddInstancedStaticMeshComponent false))
  (Components|StaticMesh|SetStaticMesh _returnvalue (Variables|Mesh|GetMesh))
  (Variables|MeshInstance|SetInstance _returnvalue)
  (if (Variables|Generate|GetShouldGenerateImmediately)
    (Generate|GenerateImmediately)))

(fn GenerateImmediately
  (for _index (range 0 (Variables|Config|GetWidthCount))
    (Generate|GenerateXStep _index)))

(fn GenerateXStep
  (params (Index :type Integer))
  (bind _objectgap (Variables|Config|GetObjectGap))
  (bind _instancearea (Variables|Measurements|GetInstanceArea))
  (bind _variance (Variables|Config|GetVariance))
  (bind _instancesize (Variables|Measurements|GetInstanceSize))
  (bind _returnvalue (/ _objectgap 2.0))
  (bind _returnvalue_2 (* _returnvalue _variance))
  (for _index (range 0 (Variables|Config|GetDepthCount))
    (for _index_2 (range 0 (Variables|Config|GetHeightCount))
      (Components|InstancedStaticMesh|AddInstance (Variables|MeshInstance|GetInstance) (Math|Transform|MakeTransform (+ (+ (+ (Math|Vector|MakeVector (+ (* (.x _instancearea) Index) (/ (.x _instancesize) 2.0)) (Math|Float|SelectFloat (* (+ (* (.y _instancearea) _index) (/ (.y _instancesize) 2.0)) -1.0) (+ (* (.y _instancearea) _index) (/ (.y _instancesize) 2.0)) (not (Variables|Config|GetFlipped))) (* _index_2 (.z _instancesize))) (Math|Vector|MakeVector (Math|Random|RandomFloatinRange (* _returnvalue_2 -1.0) _returnvalue_2) (Math|Random|RandomFloatinRange _returnvalue_2 _returnvalue_2) 0.0)) (Variables|Config|GetOriginLocation)) (Math|Vector|MakeVector (/ (.x (Variables|Measurements|GetInstanceSize)) 2.0) 0.0 0.0)) (Math|Rotator|MakeRotator 0.0 0.0 (Math|Random|RandomFloatinRange (* _returnvalue_2 -3.0) (* _returnvalue_2 3.0))))))))

(fn StartGradualGenerate
  (if (not (Variables|Generate|GetIsGraduallyGenerating))
    (Generate|ClearAllPlacedInstances)
    (Variables|Generate|SetCurrentGradualGenerateIndex 0)
    (Variables|Generate|SetIsGraduallyGenerating true)))

(fn GradualGenerateStep
  (Generate|GenerateXStep (Variables|Generate|GetCurrentGradualGenerateIndex))
  (Default|CallGenerationStep (Variables|Generate|GetCurrentGradualGenerateIndex) (Variables|Config|GetWidthCount))
  (Variables|Generate|SetCurrentGradualGenerateIndex (+ (Variables|Generate|GetCurrentGradualGenerateIndex) 1)))

(fn CheckGradualGenerateComplete
  (if (Variables|Generate|GetIsGraduallyGenerating)
    (bind _output_get (Variables|Generate|SetIsGraduallyGenerating (< (Variables|Generate|GetCurrentGradualGenerateIndex) (Variables|Config|GetWidthCount))))
    (if (not _output_get)
      (Default|CallGenerationComplete))))

(fn ClearAllPlacedInstances
  (Components|InstancedStaticMesh|ClearInstances (Variables|MeshInstance|GetInstance)))