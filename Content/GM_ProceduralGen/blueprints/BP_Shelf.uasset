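; Procedural shelf actor that builds a row of start, middle and end sections from instanced static meshes, with optional flipping.
; Construction measures mesh bounds for spacing and can generate immediately; pressing P randomizes Length and rebuilds one section per Tick.
; Both modes fire step and completion dispatchers, and GetSize reports overall dimensions plus inner shelf heights.
; The clear function empties only middle and start instances, leaving end pieces untouched.
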(event EventBeginPlay
  (Input|EnableInput (Class|GameplayStatics|GetPlayerControllerfromID)))

(event Collision|EventActorBeginOverlap
  (params (OtherActor :type Actor%20Object%20Reference)))

(event EventTick
  (params (DeltaSeconds :type Float%20%28single-precision%29))
  (if (Variables|Generate|GetIsGraduallyGenerating)
    (Generate|GradualGenerateStep)
    (Generate|CheckGradualGenerateComplete)))

(event Input|KeyboardEvents|P
  (params (Key :type Key%20Structure :default "None"))
  (:Pressed
    (if (not (Variables|Generate|GetIsGraduallyGenerating))
      (Variables|Config|SetLength (Math|Random|RandomIntegerinRange 2 10))
      (Generate|StartGradualGenerate))))

(fn ConstructionScript
  (Utilities|FlowControl|Sequence
    (:then_0
      (bind (_instance _size) (Config|InitMesh (Variables|meshes|GetShelfMesh)))
      (Variables|MeshInstance|SetShelf _instance)
      (Variables|Measurements|SetShelfSize _size)
      (bind (_instance_2 _size_2) (Config|InitMesh (Variables|Meshes|GetShelfStartMesh)))
      (Variables|MeshInstance|SetShelfStart _instance_2)
      (Variables|Measurements|SetShelfStartSize _size_2)
      (bind (_instance_3 _size_3) (Config|InitMesh (Variables|Meshes|GetShelfEndMesh)))
      (Variables|MeshInstance|SetShelfEnd _instance_3)
      (Variables|Measurements|SetShelfEndSize _size_3))
    (:then_1
      (Generate|ClearAllPlacedInstancesandMeshes)
      (if (Variables|Generate|GetShouldGenerateImmediately)
        (Generate|GenerateImmediately)))))

(fn InitMesh
  (params (Mesh :type Static%20Mesh%20Object%20Reference))
  (bind _returnvalue (AddComponent|AddInstancedStaticMeshComponent false))
  (Components|StaticMesh|SetStaticMesh _returnvalue Mesh)
  (bind _size (Utility|MeasureMesh Mesh))
  (return _returnvalue _size))

(fn MeasureMesh
  (params (mesh :type Static%20Mesh%20Object%20Reference))
  (bind _returnvalue (StaticMesh|GetBoundingBox mesh))
  (bind (_min _max) (Utilities|Struct|BreakBox _returnvalue))
  (bind _returnvalue_2 (AddComponent|AddStaticMeshComponent false))
  (Components|StaticMesh|SetStaticMesh _returnvalue_2 mesh)
  (bind _output_get (LocalVariables|SetMeshSize (- _max _min)))
  (Components|DestroyComponent _returnvalue_2)
  (return _output_get))

(fn ClearAllPlacedInstancesandMeshes
  (Components|InstancedStaticMesh|ClearInstances (Variables|MeshInstance|GetShelf))
  (Components|InstancedStaticMesh|ClearInstances (Variables|MeshInstance|GetShelfStart)))

(fn GenerateImmediately
  (bind _length (Variables|Config|GetLength))
  (for _index (range 0 _length)
    (Generate|GenerateShelfSection _index)
    (Default|CallGenerationStep _index _length))
  (Default|CallGenerationComplete))

(fn GenerateShelfSection
  (params (Index :type Integer))
  (bind _flipped (Variables|Config|GetFlipped))
  (bind _shelfsize (Variables|Measurements|GetShelfSize))
  (bind _shelfstartsize (Variables|Measurements|GetShelfStartSize))
  (bind _length (Variables|Config|GetLength))
  (bind _flipped_2 (Variables|Config|GetFlipped))
  (bind _returnvalue (Math|Float|SelectFloat 1.8e+02 0.0 _flipped))
  (bind _returnvalue_2 (Math|Float|SelectFloat -6.0 0.0 _flipped_2))
  (bind _returnvalue_3 (- _length Index))
  (bind _returnvalue_4 (- (.x _shelfsize) 3.0))
  (bind _returnvalue_5 (Math|Integer|SelectInt _returnvalue_3 Index _flipped))
  (bind _returnvalue_6 (+ (.x _shelfstartsize) _returnvalue_4))
  (bind _returnvalue_7 (Math|Float|SelectFloat _returnvalue_6 (.x _shelfstartsize) _flipped_2))
  (bind _returnvalue_8 (- _returnvalue_5 1))
  (bind _returnvalue_9 (* _returnvalue_4 _returnvalue_8))
  (bind _returnvalue_10 (+ _returnvalue_9 _returnvalue_7 _returnvalue_2))
  (bind _returnvalue_11 (Math|Transform|MakeTransform (Math|Vector|MakeVector _returnvalue_10 0.0 0.0) (Math|Rotator|MakeRotator 0.0 0.0 _returnvalue)))
  (if (== _returnvalue_5 (Math|Integer|SelectInt (Variables|Config|GetLength) 0 _flipped))
    (Components|InstancedStaticMesh|AddInstance (Variables|MeshInstance|GetShelfStart) (Math|Transform|MakeTransform (Math|Vector|MakeVector (Math|Float|SelectFloat (+ (* (- (.x (Variables|Measurements|GetShelfSize)) 3.0) (Variables|Config|GetLength)) (.x (Variables|Measurements|GetShelfStartSize))) 0.0 (Variables|Config|GetFlipped)) 0.0 0.0) (Math|Rotator|MakeRotator 0.0 0.0 _returnvalue)))
    (elif (== _returnvalue_5 (Math|Integer|SelectInt 0 (Variables|Config|GetLength) (Variables|Config|GetFlipped)))
      (Components|InstancedStaticMesh|AddInstance (Variables|MeshInstance|GetShelfEnd) _returnvalue_11)
      (else
        (Components|InstancedStaticMesh|AddInstance (Variables|MeshInstance|GetShelf) _returnvalue_11)))))

(fn StartGradualGenerate
  (if (not (Variables|Generate|GetIsGraduallyGenerating))
    (Generate|ClearAllPlacedInstancesandMeshes)
    (Variables|Generate|SetCurrentGradualGenerateIndex 0)
    (Variables|Generate|SetIsGraduallyGenerating true)))

(fn GradualGenerateStep
  (Generate|GenerateShelfSection (Variables|Generate|GetCurrentGradualGenerateIndex))
  (Default|CallGenerationStep (Variables|Generate|GetCurrentGradualGenerateIndex) (Variables|Config|GetLength))
  (Variables|Generate|SetCurrentGradualGenerateIndex (+ (Variables|Generate|GetCurrentGradualGenerateIndex) 1)))

(fn CheckGradualGenerateComplete
  (if (Variables|Generate|GetIsGraduallyGenerating)
    (bind _output_get (Variables|Generate|SetIsGraduallyGenerating (<= (Variables|Generate|GetCurrentGradualGenerateIndex) (Variables|Config|GetLength))))
    (if (not _output_get)
      (Default|CallGenerationComplete))))

(fn GetSize
  (bind _shelfsize (Variables|Measurements|GetShelfSize))
  (return (Math|Vector|MakeVector (+ (* (- (.x _shelfsize) 3.0) (- (Variables|Config|GetLength) 1)) (.x (Variables|Measurements|GetShelfStartSize)) (.x (Variables|Measurements|GetShelfEndSize))) (.y _shelfsize) (.z _shelfsize)) (Variables|Config|GetInnerShelfHeights)))