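; BP_StoreProducts is a manager actor that populates store product areas in a procedural generation setup.
; RegenerateFromAreas replaces the stored area list and AddProductsFromAreas appends to it; both spawn a tracked BP_ProductArea per supplied area and start its gradual generation.
; Spawn transforms shift back by the area's Y size when flipped on Y.
; Clearing is separate: ClearAllGenerated removes placed instances and destroys the tracked actors.
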(event EventBeginPlay)

(event Collision|EventActorBeginOverlap
  (params (OtherActor :type Actor%20Object%20Reference)))

(event EventTick
  (params (DeltaSeconds :type Float%20%28single-precision%29)))

(fn ConstructionScript)

(fn RegeneratefromAreas
  (params (Areas :type Array%20of%20S%20Shelf%20Area%20Definition%20Structures))
  (bind _output_get (Variables|Config|SetAreas Areas))
  (for _array_element _output_get
    (bind _transformresult (CallFunction|CalculateProductAreaTransform (.transform _array_element) (.size _array_element) (.isflippedony _array_element)))
    (bind _returnvalue (Game|SpawnActorfromClass "/Game/GM_ProceduralGen/blueprints/BP_ProductArea.BP_ProductArea_C" _transformresult "Undefined" 0 (.size _array_element) false 0))
    (Utilities|Array|Add (Variables|Default|GetGeneratedProductAreas) _returnvalue)
    (Default|StartGradualGenerate _returnvalue)))

(fn AddProductsfromAreas
  (params (Areas :type Array%20of%20S%20Shelf%20Area%20Definition%20Structures))
  (Utilities|Array|AppendArray (Variables|Config|GetAreas) Areas)
  (for _array_element Areas
    (bind _transformresult (CallFunction|CalculateProductAreaTransform (.transform _array_element) (.size _array_element) (.isflippedony _array_element)))
    (bind _returnvalue (Game|SpawnActorfromClass "/Game/GM_ProceduralGen/blueprints/BP_ProductArea.BP_ProductArea_C" _transformresult "Undefined" 0 (.size _array_element) false 0))
    (Utilities|Array|Add (Variables|Default|GetGeneratedProductAreas) _returnvalue)
    (Default|StartGradualGenerate _returnvalue)))

(fn ClearAllGenerated
  (bind _generatedproductareas (Variables|Default|GetGeneratedProductAreas))
  (for _array_element _generatedproductareas
    (Default|ClearAllPlacedInstances _array_element)
    (Actor|DestroyActor _array_element))
  (Utilities|Array|Clear _generatedproductareas))

(fn CalculateProductAreaTransform
  (params (InitialTransform :type Transform) (Size :type Vector) (IsFlipped :type Boolean))
  (return (Math|Transform|MakeTransform (Math|Vector|MakeVector (.x (.location InitialTransform)) (Math|Float|SelectFloat (- (.y (.location InitialTransform)) (.y Size)) (.y (.location InitialTransform)) IsFlipped) (.z (.location InitialTransform))) (.rotation InitialTransform) (.scale InitialTransform))))